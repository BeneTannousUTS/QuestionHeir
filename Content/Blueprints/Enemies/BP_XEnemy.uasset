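; BP_XEnemy is an enemy that chases the player once it sees them and can be destroyed by damage.
; PawnSensing stores a seen BP_ThirdPersonCharacter as Target and sets a chase flag that is never cleared here.
; While the flag is set, Tick reissues SimpleMoveToActor through the AI controller every frame.
; ApplyDamage subtracts from Health, printing the remainder or destroying the actor at zero or below.
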(event OnSeePawn(PawnSensing)
  (params (Pawn :type Pawn%20Object%20Reference))
  (bind _asbp_third_person_character (Utilities|Casting|CastToBP_ThirdPersonCharacter Pawn))
  (Variables|Default|SetTarget _asbp_third_person_character)
  (Variables|Default|SetbShouldChasePlayer true))

(event EventBeginPlay)

(event Collision|EventActorBeginOverlap
  (params (OtherActor :type Actor%20Object%20Reference)))

(event EventTick
  (params (DeltaSeconds :type Float%20%28single-precision%29))
  (if (Variables|Default|GetbShouldChasePlayer)
    (AI|Navigation|SimpleMovetoActor (AI|GetAIController self) (Variables|Default|GetTarget))))

(fn ConstructionScript)

(fn ApplyDamage
  (params (Damage :type Integer))
  (bind _output_get (Variables|Default|SetHealth (- (Variables|Default|GetHealth) Damage)))
  (if (<= _output_get 0)
    (Actor|DestroyActor)
    (else
      (Development|PrintString (Utilities|String|ToString(Integer) (Variables|Default|GetHealth))))))