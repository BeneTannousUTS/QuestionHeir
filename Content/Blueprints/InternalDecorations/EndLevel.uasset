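; EndLevel is an interaction point that lets the player end the game once its ShouldBecomeVisible flag is true.
; While that flag is set, Tick calls Activate on the particle system every frame.
; A player entering the sphere then gets CanInteract and CanEndGame set and sees the EPrompt.
; Leaving clears both flags and hides the prompt; this file neither sets ShouldBecomeVisible nor performs the ending.
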(event OnComponentBeginOverlap(SphereCollision)
  (params (OverlappedComponent :type Primitive%20Component%20Object%20Reference) (OtherActor :type Actor%20Object%20Reference) (OtherComp :type Primitive%20Component%20Object%20Reference) (OtherBodyIndex :type Integer) (bFromSweep :type Boolean) (SweepResult :type Hit%20Result%20Structure%20%28by%20ref%29))
  (bind _eprompt (Variables|Default|GetEPrompt))
  (if (Variables|Default|GetbShouldBecomeVisible)
    (bind _asbp_third_person_character (Utilities|Casting|CastToBP_ThirdPersonCharacter OtherActor))
    (bind _output_get (Variables|Default|SetOverlappedPlayer _asbp_third_person_character))
    (Variables|/Game/ThirdPerson/Blueprints/BP_ThirdPersonCharacter.BP_ThirdPersonCharacter_C|SetbCanInteract _asbp_third_person_character true)
    (Variables|/Game/ThirdPerson/Blueprints/BP_ThirdPersonCharacter.BP_ThirdPersonCharacter_C|SetbCanEndGame _output_get true)
    (if (Utilities|IsValid _eprompt)
      (Development|SetHiddeninGame _eprompt false false))))

(event OnComponentEndOverlap(SphereCollision)
  (params (OverlappedComponent :type Primitive%20Component%20Object%20Reference) (OtherActor :type Actor%20Object%20Reference) (OtherComp :type Primitive%20Component%20Object%20Reference) (OtherBodyIndex :type Integer))
  (bind _eprompt (Variables|Default|GetEPrompt))
  (bind _asbp_third_person_character (Utilities|Casting|CastToBP_ThirdPersonCharacter OtherActor))
  (Variables|/Game/ThirdPerson/Blueprints/BP_ThirdPersonCharacter.BP_ThirdPersonCharacter_C|SetbCanInteract _asbp_third_person_character false)
  (Variables|/Game/ThirdPerson/Blueprints/BP_ThirdPersonCharacter.BP_ThirdPersonCharacter_C|SetbCanEndGame _asbp_third_person_character false)
  (if (Utilities|IsValid _eprompt)
    (Development|SetHiddeninGame _eprompt true false)))

(event EventBeginPlay)

(event Collision|EventActorBeginOverlap
  (params (OtherActor :type Actor%20Object%20Reference)))

(event EventTick
  (params (DeltaSeconds :type Float%20%28single-precision%29))
  (if (Variables|Default|GetbShouldBecomeVisible)
    (Components|Activation|Activate (Variables|Default|GetParticleSystem) false)))

(fn ConstructionScript)