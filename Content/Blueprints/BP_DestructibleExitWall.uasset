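; BP_DestructibleExitWall is a wall the player can blow open, presumably as an exit.
; A proximity sphere shows the E prompt and gives the third-person character interaction permission and a reference to this wall.
; DoorExplosion destroys the wall mesh and prompt, playing explosion and rockfall particles and sounds.
; Tick then uses an accumulated timer to start smoke after a short delay and stop it seconds later.
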(event OnComponentBeginOverlap(SphereCollision)
  (params (OverlappedComponent :type Primitive%20Component%20Object%20Reference) (OtherActor :type Actor%20Object%20Reference) (OtherComp :type Primitive%20Component%20Object%20Reference) (OtherBodyIndex :type Integer) (bFromSweep :type Boolean) (SweepResult :type Hit%20Result%20Structure%20%28by%20ref%29))
  (bind _eprompt (Variables|Default|GetEPrompt))
  ;[1 1 1] Player Proximity logic
  (bind _asbp_third_person_character (Utilities|Casting|CastToBP_ThirdPersonCharacter OtherActor))
  (bind _output_get (Variables|Default|SetOverlappedPlayer _asbp_third_person_character))
  (Variables|/Game/ThirdPerson/Blueprints/BP_ThirdPersonCharacter.BP_ThirdPersonCharacter_C|SetbCanInteract _output_get true)
  (Variables|/Game/ThirdPerson/Blueprints/BP_ThirdPersonCharacter.BP_ThirdPersonCharacter_C|SetDoorReference _output_get self)
  (if (Utilities|IsValid _eprompt)
    (Development|SetHiddeninGame _eprompt false false)))

(event OnComponentEndOverlap(SphereCollision)
  (params (OverlappedComponent :type Primitive%20Component%20Object%20Reference) (OtherActor :type Actor%20Object%20Reference) (OtherComp :type Primitive%20Component%20Object%20Reference) (OtherBodyIndex :type Integer))
  (bind _eprompt (Variables|Default|GetEPrompt))
  ;[1 1 1] Player Proximity logic
  (bind _asbp_third_person_character (Utilities|Casting|CastToBP_ThirdPersonCharacter OtherActor))
  (Variables|/Game/ThirdPerson/Blueprints/BP_ThirdPersonCharacter.BP_ThirdPersonCharacter_C|SetbCanInteract _asbp_third_person_character false)
  (if (Utilities|IsValid _eprompt)
    (Development|SetHiddeninGame _eprompt true false)))

(event EventBeginPlay)

(event Collision|EventActorBeginOverlap
  (params (OtherActor :type Actor%20Object%20Reference)))

(event EventTick
  (params (DeltaSeconds :type Float%20%28single-precision%29))
  (if (Variables|Default|GetbCanFullyDestroy)
    (bind _output_get (Variables|Default|SetSmokeDelay (+ DeltaSeconds (Variables|Default|GetSmokeDelay))))
    (if (> _output_get 0.3)
      (CallFunction|PostExplosionSmoke)
      (if (> _output_get 5.0)
        (Components|Activation|Deactivate (Variables|Default|GetP_Smoke))
        (Variables|Default|SetbCanFullyDestroy false)))))

(fn ConstructionScript)

(fn DoorExplosion
  (bind _p_explosion (Variables|Default|GetP_Explosion))
  (bind _p_rocktumble (Variables|Default|GetP_RockTumble))
  (Components|Activation|Activate _p_explosion true)
  (Components|DestroyComponent (Variables|Default|GetWallMesh))
  (Audio|PlaySoundatLocation "/Game/StarterContent/Audio/Explosion_Cue.Explosion_Cue" (Transformation|GetWorldLocation _p_explosion) "0, 0, 0" 1.0 1.0 0.0 0 0 0 0)
  (Components|DestroyComponent (Variables|Default|GetEPrompt))
  (Components|Activation|Activate _p_rocktumble true)
  (Audio|PlaySoundatLocation "/Game/Audio/SFX/SC_DoorRockFall.SC_DoorRockFall" (Transformation|GetWorldLocation _p_rocktumble) "0, 0, 0" 1.0 1.0 0.0 0 0 0 0)
  (Variables|Default|SetbCanFullyDestroy true))

(fn PostExplosionSmoke
  (Components|Activation|Activate (Variables|Default|GetP_Smoke) false))

(fn DestroyDoor)